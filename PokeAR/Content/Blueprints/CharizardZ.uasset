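; Charizard character actor that plays a looping waiting animation and exposes events for fireball attack and hit reactions.
; The fireball event reveals FireBall and Sphere partway through the attack animation, then hides them and activates particle and audio components when it ends.
; While the fireball is visible, Tick moves GeometryCache and spins both meshes, otherwise resetting its position.
; Both events poll IsPlaying through Delay loops before returning to waiting.
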(event Custom|Start%20TakingDamage%20Animation
  (bind _skeletalmesh (Variables|Default|GetSkeletalMesh))
  (Components|Animation|PlayAnimation _skeletalmesh "/Game/HandheldARBP/Charizard/charizardV16_Anim_Armature_001_Armature_Hit.charizardV16_Anim_Armature_001_Armature_Hit" false)
  (if (Audio|Components|Audio|IsPlaying _skeletalmesh) :!label _label
    (Utilities|FlowControl|Delay 0.2)
    (goto _label)
    (else
      (Components|Animation|PlayAnimation (Variables|Default|GetSkeletalMesh) "/Game/HandheldARBP/Charizard/charizardV16_Anim_Armature_001_Armature_Waiting.charizardV16_Anim_Armature_001_Armature_Waiting" true))))

(event Custom|Start%20FireBall%20Animation
  (bind _skeletalmesh (Variables|Default|GetSkeletalMesh))
  (bind _returnvalue (Audio|Components|Audio|IsPlaying _skeletalmesh))
  (Components|Animation|PlayAnimation _skeletalmesh "/Game/HandheldARBP/Charizard/charizardV16_Anim_Armature_001_Armature_Fireball.charizardV16_Anim_Armature_001_Armature_Fireball" false)
  (if _returnvalue
    (Utilities|FlowControl|Delay 1.5)
    (Rendering|SetVisibility (Variables|Default|GetFireBall) true false)
    (if _returnvalue :!label _label
      (Utilities|FlowControl|Delay 0.2)
      (goto _label)
      (else
        (Rendering|SetVisibility (Variables|Default|GetFireBall) false false)
        (Components|Animation|PlayAnimation (Variables|Default|GetSkeletalMesh) "/Game/HandheldARBP/Charizard/charizardV16_Anim_Armature_001_Armature_Waiting.charizardV16_Anim_Armature_001_Armature_Waiting" true)
        (Components|Activation|Activate (Variables|Default|GetParticleSystem) false)))))

(event EventBeginPlay
  (Components|Animation|PlayAnimation (Variables|Default|GetSkeletalMesh) "/Game/HandheldARBP/Charizard/charizardV16_Anim_Armature_001_Armature_Waiting.charizardV16_Anim_Armature_001_Armature_Waiting" true))

(event EventTick
  (params (DeltaSeconds :type Float%20%28single-precision%29))
  (bind _geometrycache (Variables|Default|GetGeometryCache))
  (if (Rendering|IsVisible (Variables|Default|GetFireBall))
    (Transformation|AddLocalOffset _geometrycache "0,25.000000, 0" false false)
    (Transformation|AddLocalRotation (Variables|Default|GetSphere) "10.000000,10.000000,10.000000" false false)
    (else
      (Transformation|SetRelativeLocation _geometrycache "-240.000000,40.000000,100.000000" false false))))

(fn ConstructionScript)